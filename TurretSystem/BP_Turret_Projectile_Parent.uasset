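; Parent projectile Blueprint for the turret system that damages test dummies on overlap and then destroys itself.
; Projectile movement bounce events count down a bounce budget set on BeginPlay, destroying the projectile once it runs out.
; Tick also destroys it once its straight-line distance from the start location reaches ProjectileRange.
; A Reflect event redirects it by overwriting its velocity along a given direction at fixed speed.
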(event `self.ReceiveActorBeginOverlap`
  (params (OtherActor :type "Actor Object Reference"))
  (bind _astest_dummy (cast `/Game/Enemies/TestDummy` OtherActor))
  (`TestDummyEnemy.TakeDamage` (`/Game/Enemies/TestDummy.TestDummyEnemy` _astest_dummy) 15.0)
  (`self.K2_DestroyActor`))

(event `self.ProjectileMovement.OnProjectileBounce`
  (params (ImpactResult :type "HitResult Structure (by ref)") (ImpactVelocity :type "Vector Structure (by ref)"))
  (bind _numbounces (`self.numBounces`))
  ;[1 1 1] Checking if projectile bounced using bounce method from unreal and reduces number of bounces. If bounces are zero, destroys. We should later set up a collision preset so we can use specific collision meshes as bounceable and not deal with all unreals collision setting shit.
  (if (<= _numbounces 0)
    (`self.K2_DestroyActor`)
    (else
      (set `self.numBounces` (- _numbounces 1)))))

(event `self.ReceiveBeginPlay`
  (set `self.startlocation` (`self.K2_GetActorLocation`))
  (set `self.numBounces` 5))

(event `self.ReceiveTick`
  (params (DeltaSeconds :type "Float (single-precision)"))
  (if (>= (`KismetMathLibrary.VSize` (- (`self.startlocation`) (`self.K2_GetActorLocation`))) (`self.projectileRange`))
    (`/Engine/EditorBlueprintResources/StandardMacros.DoOnce` false
      (:`Completed`
        (`self.K2_DestroyActor`)))))

(event `self.Reflect`
  (params (direction :type "Vector Structure"))
  (set `MovementComponent.Velocity` (* direction 2000) (`self.ProjectileMovement`)))

(fn `UserConstructionScript`)