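; Turret actor that tracks the player character and fires projectiles from its cannon.
; Each Tick it checks range to the player's camera, then either turns base yaw and platform pitch toward it at constant interpolation speed or eases back to neutral.
; Close alignment passes a DoOnce into StartFiring, where the TurretRefire timeline acts as a self-repeating refire timer.
; StopFiring only clears CanShoot, which that repeat path does not recheck.
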(event `self.ReceiveActorBeginOverlap`
  (params (OtherActor :type "Actor Object Reference"))
  (if (== (`GameplayStatics.GetObjectClass` OtherActor) "/Game/TurretSystem/BP_Turret/BP_Turret_Projectile_Parent.BP_Turret_Projectile_Parent_C")
    _))

(event `FireProjectile`
  ;[1 1 1] Fire at player
  (`|SpawnActorFromClass` "/Game/TurretSystem/BP_Turret/BP_Turret_Projectile_Parent.BP_Turret_Projectile_Parent_C" (`KismetMathLibrary.MakeTransform` (.location (`SceneComponent.K2_GetComponentToWorld` (`self.CannonMesh`))) (.rotation (`SceneComponent.K2_GetComponentToWorld` (`self.CannonMesh`))) (0.25 0.25 0.25)) "Undefined" "OverrideRootScale" null null))

(event `StartFiring`
  ;[1 1 1] Fire at player
  (if (`self.CanShoot`)
    (if (== (`TimelineComponent.GetPlaybackPosition` (`self.TurretRefire`)) 0.0) :!label _label
      (`self.FireProjectile`)
      (`Timeline|TurretRefire` :!label _label_2
        (:`Finished`
          (`self.ResetFireTimeline`)
          (`self.ContinueFiring`))))))

(event `ContinueFiring`
  ;[1 1 1] Fire at player
  (`TimelineComponent.SetTimelineLength` (`self.TurretRefire`) (`self.RefireDelay`))
  (goto _label))

(event `ResetFireTimeline`
  ;[1 1 1] Fire at player
  (`|ExecutionSequence`
    (:`then_0`
      (goto _label_2 :!via `Stop`))
    (:`then_1`
      (goto _label_2 :!via `SetNewTime`))))

(event `StopFiring`
  ;[1 1 1] Fire at player
  (set `self.CanShoot` false))

(event `self.ReceiveBeginPlay`
  ;[1 1 1] Gets the target player
  (bind _outactors (`GameplayStatics.GetAllActorsOfClass` "/Script/HellOfARacket.CustomHellRacketCharacter"))
  (set `self.Target` (`|GetArrayItem` _outactors)))

(event `self.ReceiveTick`
  (params (DeltaSeconds :type "Float (single-precision)"))
  ;[1 1 1] Get Target/Players Location
  (set `self.TargetLocation` (`SceneComponent.K2_GetComponentLocation` (`CustomHellRacketCharacter.cam` (`self.Target`))))
  ;[1 1 1] Check target distance
  (if (<= (`KismetMathLibrary.VSize` (- (`self.K2_GetActorLocation`) (`self.TargetLocation`))) 2000.0)
    ;[1 1 1] Trigger events
    (`self.Aim at target`)
    (else
      (`self.Reset Target`)
      (`self.StopFiring`))))

(event `Aim at target`
  (bind _returnvalue (`KismetMathLibrary.FindLookAtRotation` (`SceneComponent.K2_GetComponentLocation` (`self.PlatformMesh`)) (`self.TargetLocation`)))
  ;[1 1 1] Setting the rotation of the turret to face the player
  (set `self.TargetAimRotator` _returnvalue)
  (`SceneComponent.K2_SetRelativeRotation` (`self.BaseMesh`) (`KismetMathLibrary.RInterpTo_Constant` (`SceneComponent.RelativeRotation` (`self.BaseMesh`)) (`KismetMathLibrary.MakeRotator` 0.0 0.0 (.yaw _returnvalue)) (`GameplayStatics.GetWorldDeltaSeconds`) (`self.SpeedofRotation`)) false false)
  ;;[1 1 1] Comment
  (`SceneComponent.K2_SetRelativeRotation` (`self.PlatformMesh`) (`KismetMathLibrary.RInterpTo_Constant` (`SceneComponent.RelativeRotation` (`self.PlatformMesh`)) (`KismetMathLibrary.MakeRotator` 0.0 (.pitch _returnvalue)) (`GameplayStatics.GetWorldDeltaSeconds`) (`self.SpeedofRotation`)) false false)
  ;;[1 1 1] This is checking of the turret is looking close enough to fire at the character
  (if (== (`self.TargetAimRotator`) (`KismetMathLibrary.MakeRotator` 0.0 (.pitch (`SceneComponent.RelativeRotation` (`self.PlatformMesh`))) (.yaw (`SceneComponent.RelativeRotation` (`self.BaseMesh`)))) :`ErrorTolerance` 1.0)
    (`|ExecutionSequence`
      (:`then_0`
        (`/Engine/EditorBlueprintResources/StandardMacros.DoOnce` false :!label _label_3
          (:`Completed`
            (set `self.CanShoot` true)
            (`self.StartFiring`)))))
    (else
      (`self.StopFiring`))))

(event `ResetFireTrigger`
  ;[1 1 1] Setting the rotation of the turret to face the player
  ;;[1 1 1] This is checking of the turret is looking close enough to fire at the character
  (goto _label_3 :!via `Reset`))

(event `Reset Target`
  ;[1 1 1] If the player leaves the area of the turret the rotation gets set back to where it started
  (`SceneComponent.K2_SetRelativeRotation` (`self.BaseMesh`) (`KismetMathLibrary.RInterpTo_Constant` (`SceneComponent.RelativeRotation` (`self.BaseMesh`)) (`KismetMathLibrary.MakeRotator` 0.0) (`GameplayStatics.GetWorldDeltaSeconds`) 75.0) false false)
  (`SceneComponent.K2_SetRelativeRotation` (`self.PlatformMesh`) (`KismetMathLibrary.RInterpTo_Constant` (`SceneComponent.RelativeRotation` (`self.PlatformMesh`)) (`KismetMathLibrary.MakeRotator` 0.0) (`GameplayStatics.GetWorldDeltaSeconds`) 75.0) false false))

(fn `UserConstructionScript`)